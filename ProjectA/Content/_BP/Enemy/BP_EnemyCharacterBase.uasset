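; Base enemy character Blueprint that handles the death sequence through a dissolve effect.
; On death it freezes animation, disables capsule collision, removes the enemy UI widget and async-loads a Niagara effect attached to the mesh.
; The particles take the material's dissolve edge color, while a timeline scaled by dissolve time drives DissolveAmount on the mesh and equipped weapon, then destroys both.
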(event `self.ReceiveBeginPlay`)

(event `/Game/_BP/Enemy/MeleeMonster/BPI_Enemy_Death.OnEnemyDie`
  (params (VFX :type "NiagaraSystem Soft Object Reference"))
  (bind _mesh (`self.Mesh`))
  (bind _returnvalue (`PawnCombatComponent.GetCharacterCurrentEquippedWeapon` (`self.EnemyCombatComponent`)))
  (bind _returnvalue_2 (`PawnCombatComponent.GetCharacterCurrentEquippedWeapon` (`self.EnemyCombatComponent`)))
  (`|ExecutionSequence`
    (:`then_0`
      (set `SkeletalMeshComponent.bPauseAnims` true (`self.Mesh`))
      (`PrimitiveComponent.SetCollisionEnabled` (`self.CapsuleComponent`) "NoCollision"))
    (:`then_1`
      (`EnemyUIComponent.RemoveEnemyWidget` (`self.EnemyUIComponent`)))
    (:`then_2`
      (bind _object (`|LoadAsset` VFX)
        (:`Completed`
          (bind _asniagara_system (cast `NiagaraSystem` _object))
          (bind _returnvalue_3 (`NiagaraFunctionLibrary.SpawnSystemAttached` _asniagara_system (`self.Mesh`) "None" (0.0 0.0 0.0) (struct) "KeepRelativeOffset"))
          (bind _returnvalue_4 (`PrimitiveComponent.CreateDynamicMaterialInstance` _mesh 0 (`PrimitiveComponent.GetMaterial` _mesh 0) "None"))
          (bind _returnvalue_5 (`MaterialInstanceDynamic.K2_GetVectorParameterValue` _returnvalue_4 "DissolveEdgeColor"))
          (`NiagaraComponent.SetNiagaraVariableLinearColor` _returnvalue_3 "DissolveParticleColor" _returnvalue_5)
          (`TimelineComponent.SetPlayRate` (`self.DessolveTimeline`) (/ 1.0 (`self.DessolveTime`)))
          (bind (_direction _normalizedfloat) (`Timeline|DessolveTimeline` :!via `PlayFromStart`)
            (:`Update`
              (`MeshComponent.SetScalarParameterValueOnMaterials` (`self.Mesh`) "DissolveAmount" _normalizedfloat)
              (`/Engine/EditorBlueprintResources/StandardMacros.IsValid` _returnvalue_2
                (:`Is Valid`
                  (`MeshComponent.SetScalarParameterValueOnMaterials` (`WeaponBase.WeaponMesh` _returnvalue_2) "DissolveAmount" _normalizedfloat))))
            (:`Finished`
              (`/Engine/EditorBlueprintResources/StandardMacros.IsValid` _returnvalue
                (:`Is Valid`
                  (`self.K2_DestroyActor` _returnvalue))
                (:`Is Not Valid`
                  _))
              (`self.K2_DestroyActor`))))))))

(fn `UserConstructionScript`)