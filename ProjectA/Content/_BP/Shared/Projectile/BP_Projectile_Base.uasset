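; BP_Projectile_Base is a projectile base Blueprint that handles launch, flight and impact audio and visual effects.
; On BeginPlay it plays FlySound both at the spawn location and attached to the root, stopping with it, and spawns a forward-facing muzzle Niagara effect.
; OnSpawnProjectileHitFX plays a sound and spawns a Niagara system at the supplied hit location.
; Each effect is skipped if its asset is unset.
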(event `self.ReceiveBeginPlay`
  (`|ExecutionSequence`
    (:`then_0`
      (bind _flysound (`self.FlySound`)
        (:`then`
          (`GameplayStatics.PlaySoundAtLocation` _flysound (`self.K2_GetActorLocation`) (struct) 1.0 1.0 0.0 null null null null))
        (:`else`)))
    (:`then_1`
      (bind _flysound_2 (`self.FlySound`)
        (:`then`
          (`GameplayStatics.SpawnSoundAttached` _flysound_2 (`self.RootComponent`) "None" (0.0 0.0 0.0) (struct) "KeepRelativeOffset" true 1.0 1.0 0.0 null null))
        (:`else`)))
    (:`then_2`
      (bind _projectilemuzzlefx (`self.ProjectileMuzzleFX`)
        (:`then`
          (`NiagaraFunctionLibrary.SpawnSystemAtLocation` _projectilemuzzlefx (`self.K2_GetActorLocation`) (`KismetMathLibrary.Conv_VectorToRotator` (`self.GetActorForwardVector`))))
        (:`else`)))))

(event `self.BP_OnSpawnProjectileHitFX`
  (params (HitLocation :type "Vector Structure (by ref)"))
  (`|ExecutionSequence`
    (:`then_0`
      (bind _sound (`self.Sound`)
        (:`then`
          (`GameplayStatics.PlaySoundAtLocation` _sound HitLocation (struct) 1.0 1.0 0.0 null null null null))
        (:`else`)))
    (:`then_1`
      (bind _system_template (`self.System Template`)
        (:`then`
          (`NiagaraFunctionLibrary.SpawnSystemAtLocation` _system_template HitLocation))
        (:`else`)))))

(fn `UserConstructionScript`)